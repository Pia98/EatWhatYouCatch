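; Game manager for a timed mixed-reality pizza game where random toppings rain from a spawn volume.
; BeginPlay starts AR scene capture, spawns the pizza and starts music.
; Tick feeds the countdown to the MR pawn's UI and a frame-counted spawn timer, while DestroyArea removes overlapping food.
; Shape, type and mesh use separate Selects over a random 0–4 range, leaving the sixth option unreachable.
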(event `self.ReceiveBeginPlay`
  ;[1 1 1] game start
  (if (`MicrosoftOpenXRFunctionLibrary.CanDetectPlanes`)
    (`ARBlueprintLibrary.ToggleARCapture` true "SceneUnderstanding")
    (else
      (`ARBlueprintLibrary.ToggleARCapture` true "SpatialMapping")))
  (set `self.TimeRemaining` (`self.TimerDuration`))
  (set `self.SpawnTimer` (`self.DurationBetweenSpawns`))
  (`|SpawnActorFromClass` "/Game/Blueprints/Pizza.Pizza_C" (`KismetMathLibrary.MakeTransform` (50.0 0.0 0.0) (struct :`Roll` 90.0) (0.4 0.4 0.4)) "AlwaysSpawn" "OverrideRootScale" null null)
  (`GameplayStatics.PlaySound2D` "/Game/Sound/music2.music2" 0.8 1.0 0.0 null null))

(event `self.ReceiveTick`
  (params (DeltaSeconds :type "Float (single-precision)"))
  ;[1 1 1] update game
  (`self.UpdateGame`))

(event `self.DestroyArea.OnComponentBeginOverlap`
  (params (OverlappedComponent :type "PrimitiveComponent Object Reference") (OtherActor :type "Actor Object Reference") (OtherComp :type "PrimitiveComponent Object Reference") (OtherBodyIndex :type Integer) (bFromSweep :type Boolean) (SweepResult :type "HitResult Structure (by ref)"))
  (bind _asfood (cast `/Game/Blueprints/Food` OtherActor))
  (`self.K2_DestroyActor` _asfood))

(fn `checkSpawnTimer`
  (bind _durationbetweenspawns (`self.DurationBetweenSpawns`))
  (set `self.SpawnTimer` (- (`self.SpawnTimer`) 1.0))
  (if (>= 0.0 (`self.SpawnTimer`))
    (`self.spawn`)
    (set `self.SpawnTimer` _durationbetweenspawns)
    (`KismetSystemLibrary.PrintString` "Spawn")
    (`KismetSystemLibrary.PrintString` (`KismetStringLibrary.Conv_DoubleToString` _durationbetweenspawns))))

(fn `spawn`
  (bind _returnvalue (`KismetMathLibrary.RandomIntegerInRange` 0 4))
  (bind (_origin _boxextent) (`KismetSystemLibrary.GetComponentBounds` (`self.SpawnArea`)))
  (bind _returnvalue_2 (select `int` _returnvalue :`0` "/Game/Mesh/Cheese.Cheese" :`1` "/Game/Mesh/Mozarella.Mozarella" :`2` "/Game/Mesh/Olive.Olive" :`3` "/Game/Mesh/Salami.Salami" :`4` "/Game/Mesh/Tomate.Tomate" :`5` "/Game/Mesh/Rokula.Rokula" :!type "StaticMesh Object Reference"))
  (bind _returnvalue_3 (`|SpawnActorFromClass` "/Game/Blueprints/Food.Food_C" (`KismetMathLibrary.MakeTransform` (`KismetMathLibrary.RandomPointInBoundingBox` _origin _boxextent) (struct :`Roll` 90.0) (1.5 1.5 1.5)) "Undefined" "OverrideRootScale" null null))
  (set `/Game/Blueprints/Food.Mesh Shape` _returnvalue_2 _returnvalue_3)
  (set `/Game/Blueprints/Food.type` (select `int` _returnvalue :`0` "NewEnumerator4" :`1` "NewEnumerator5" :`2` "NewEnumerator2" :`3` "NewEnumerator1" :`4` "NewEnumerator0" :`5` "NewEnumerator3" :!type "/Game/Blueprints/Products Enum") _returnvalue_3)
  (`StaticMeshComponent.SetStaticMesh` (`/Game/Blueprints/Food.StaticMesh` _returnvalue_3) _returnvalue_2))

(fn `UpdateGame`
  ;[0.5059 1 0.7143] if there is still time remaining continue spawning
  (if (>= (`self.TimeRemaining`) 0.0)
    (`|ExecutionSequence`
      (:`then_0`
        (`self.updateTimer`))
      (:`then_1`
        (`self.checkSpawnTimer`)))))

(fn `updateTimer`
  (set `self.TimeRemaining` (`KismetMathLibrary.FClamp` (- (`self.TimeRemaining`) (`GameplayStatics.GetWorldDeltaSeconds`)) 0.0 100.0))
  (bind _asmrpawn (cast `/Game/Blueprints/MRPawn` (`GameplayStatics.GetPlayerPawn` 0)))
  (`/Game/UI/UIStatus.set timer_text` (`/Game/Blueprints/MRPawn.uistatus` _asmrpawn) (`self.TimeRemaining`)))

(fn `UserConstructionScript`)