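; Pizza actor for a mixed reality catching game: the pizza shows on the player's upturned palm and collects Food ingredients.
; UxtPalmUpConstraint toggles the mesh's visibility and query collision as the constraint activates and deactivates.
; On overlap it raises total and per-type counts, updates the MRPawn's Uistatus, destroys the food and plays a sound.
; The Morzarella case increments OliveCount, so it shares the olive tally.
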(event `self.ReceiveActorBeginOverlap`
  (params (OtherActor :type "Actor Object Reference"))
  (bind _asfood (cast `/Game/Blueprints/Food` OtherActor))
  (if (== (`GameplayStatics.GetObjectClass` OtherActor) "/Game/Blueprints/Food.Food_C")
    (bind _result (`/Engine/EditorBlueprintResources/StandardMacros.IncrementInt` (`self.foodCount`))
      (:`  `
        (bind _output_get (set `self.foodCount` _result))
        (`KismetSystemLibrary.PrintString` (`KismetStringLibrary.Conv_IntToString` _output_get))
        (bind _asmrpawn (cast `/Game/Blueprints/MRPawn` (`GameplayStatics.GetPlayerPawn` 0))
          (:`then`
            (bind _uistatus (`/Game/Blueprints/MRPawn.uistatus` _asmrpawn))
            (`/Game/UI/UIStatus.set itemCount_Text` _uistatus (`self.foodCount`))
            (bind _type (`/Game/Blueprints/Food.type` _asfood))
            (switch `/Game/Blueprints/Products` _type
              (:`NewEnumerator0`
                (bind _result_2 (`/Engine/EditorBlueprintResources/StandardMacros.IncrementInt` (`self.tomatoCount`))
                  (:`  `
                    (`/Game/UI/UIStatus.set product_text` _uistatus _type _result_2))))
              (:`NewEnumerator1`
                (bind _result_3 (`/Engine/EditorBlueprintResources/StandardMacros.IncrementInt` (`self.salamiCount`))
                  (:`  `
                    (`/Game/UI/UIStatus.set product_text` _uistatus _type _result_3))))
              (:`NewEnumerator2`
                (bind _result_4 (`/Engine/EditorBlueprintResources/StandardMacros.IncrementInt` (`self.oliveCount`))
                  (:`  `
                    (`/Game/UI/UIStatus.set product_text` _uistatus _type _result_4))))
              (:`NewEnumerator3`
                (bind _result_5 (`/Engine/EditorBlueprintResources/StandardMacros.IncrementInt` (`self.rucolaCount`))
                  (:`  `
                    (`/Game/UI/UIStatus.set product_text` _uistatus _type _result_5))))
              (:`NewEnumerator4`
                (bind _result_6 (`/Engine/EditorBlueprintResources/StandardMacros.IncrementInt` (`self.cheeseCount`))
                  (:`  `
                    (`/Game/UI/UIStatus.set product_text` _uistatus _type _result_6))))
              (:`NewEnumerator5`
                (bind _result_7 (`/Engine/EditorBlueprintResources/StandardMacros.IncrementInt` (`self.oliveCount`))
                  (:`  `
                    (`/Game/UI/UIStatus.set product_text` _uistatus _type _result_7))))))
          (:`CastFailed`
            _))
        (`self.K2_DestroyActor` OtherActor)
        (`GameplayStatics.PlaySound2D` "/Game/Sound/caught_sound.caught_sound" 1.0 1.0 0.0 null null)))))

(event `self.UxtPalmUpConstraint.OnConstraintActivated`
  (`SceneComponent.SetVisibility` (`self.PizzaMesh`) true false)
  (`PrimitiveComponent.SetCollisionEnabled` (`self.PizzaMesh`) "QueryOnly"))

(event `self.UxtPalmUpConstraint.OnConstraintDeactivated`
  (`SceneComponent.SetVisibility` (`self.PizzaMesh`) false false)
  (`PrimitiveComponent.SetCollisionEnabled` (`self.PizzaMesh`) "NoCollision"))

(fn `UserConstructionScript`)