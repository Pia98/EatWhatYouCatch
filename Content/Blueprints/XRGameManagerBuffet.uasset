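; Game manager for a timed XR pizza-topping buffet that starts AR capture, spawns the pizza and plays music.
; Tick counts down the round on the MRPawn's UI and, on a frame-counted interval, spawns five topping types at random points within their area components.
; At zero it spawns an EndGame button and refills the timer, so spawning resumes.
; A DestroyArea overlap removes Food and EndGame actors.
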(event `self.ReceiveBeginPlay`
  ;[1 1 1] game start
  (if (`MicrosoftOpenXRFunctionLibrary.CanDetectPlanes`)
    (`ARBlueprintLibrary.ToggleARCapture` true "SceneUnderstanding")
    (else
      (`ARBlueprintLibrary.ToggleARCapture` true "SpatialMapping")))
  (set `self.TimeRemaining` (`self.TimerDuration`))
  (set `self.SpawnTimer` (`self.DurationBetweenSpawns`))
  (`|SpawnActorFromClass` "/Game/Blueprints/Pizza.Pizza_C" (`KismetMathLibrary.MakeTransform` (50.0 0.0 0.0) (struct :`Roll` 90.0) (0.4 0.4 0.4)) "AlwaysSpawn" "OverrideRootScale" null null)
  (`GameplayStatics.PlaySound2D` "/Game/Sound/music2.music2" 0.8 1.0 0.0 null null))

(event `self.ReceiveTick`
  (params (DeltaSeconds :type "Float (single-precision)"))
  ;[1 1 1] update game
  (`self.Update Game`))

(event `self.DestroyArea.OnComponentBeginOverlap`
  (params (OverlappedComponent :type "PrimitiveComponent Object Reference") (OtherActor :type "Actor Object Reference") (OtherComp :type "PrimitiveComponent Object Reference") (OtherBodyIndex :type Integer) (bFromSweep :type Boolean) (SweepResult :type "HitResult Structure (by ref)"))
  (bind _returnvalue (`GameplayStatics.GetObjectClass` OtherActor))
  (if (or (== _returnvalue "/Game/Blueprints/Food.Food_C") (== _returnvalue "/Game/Blueprints/EndGame.EndGame_C"))
    (`self.K2_DestroyActor` OtherActor)))

(fn `checkSpawnTimer`
  (set `self.SpawnTimer` (- (`self.SpawnTimer`) 1.0))
  (if (>= 0.0 (`self.SpawnTimer`))
    (`self.spawn`)
    (set `self.SpawnTimer` (`self.DurationBetweenSpawns`))))

(fn `spawn`
  (bind (_origin _boxextent) (`KismetSystemLibrary.GetComponentBounds` (`self.OliveArea`)))
  (bind (_origin_2 _boxextent_2) (`KismetSystemLibrary.GetComponentBounds` (`self.MorzarellaArea`)))
  (bind (_origin_3 _boxextent_3) (`KismetSystemLibrary.GetComponentBounds` (`self.SalamiArea`)))
  (bind (_origin_4 _boxextent_4) (`KismetSystemLibrary.GetComponentBounds` (`self.TomatoArea`)))
  (bind (_origin_5 _boxextent_5) (`KismetSystemLibrary.GetComponentBounds` (`self.CheeseArea`)))
  (`|ExecutionSequence`
    (:`then_0`
      (bind _returnvalue (`|SpawnActorFromClass` "/Game/Blueprints/Food.Food_C" (`KismetMathLibrary.MakeTransform` (`KismetMathLibrary.RandomPointInBoundingBox` _origin_4 _boxextent_4) (struct :`Roll` 90.0) (1.5 1.5 1.5)) "Undefined" "OverrideRootScale" null null))
      (bind _output_get (set `/Game/Blueprints/Food.Mesh Shape` "/Game/Mesh/Tomate.Tomate" _returnvalue))
      (set `/Game/Blueprints/Food.type` "NewEnumerator0" _returnvalue)
      (`StaticMeshComponent.SetStaticMesh` (`/Game/Blueprints/Food.StaticMesh` _returnvalue) _output_get))
    (:`then_1`
      (bind _returnvalue_2 (`|SpawnActorFromClass` "/Game/Blueprints/Food.Food_C" (`KismetMathLibrary.MakeTransform` (`KismetMathLibrary.RandomPointInBoundingBox` _origin_5 _boxextent_5) (struct :`Roll` 90.0) (1.5 1.5 1.5)) "Undefined" "OverrideRootScale" null null))
      (bind _output_get_2 (set `/Game/Blueprints/Food.Mesh Shape` "/Game/Mesh/Cheese.Cheese" _returnvalue_2))
      (set `/Game/Blueprints/Food.type` "NewEnumerator4" _returnvalue_2)
      (`StaticMeshComponent.SetStaticMesh` (`/Game/Blueprints/Food.StaticMesh` _returnvalue_2) _output_get_2))
    (:`then_2`
      (bind _returnvalue_3 (`|SpawnActorFromClass` "/Game/Blueprints/Food.Food_C" (`KismetMathLibrary.MakeTransform` (`KismetMathLibrary.RandomPointInBoundingBox` _origin_2 _boxextent_2) (struct :`Roll` 90.0) (1.5 1.5 1.5)) "Undefined" "OverrideRootScale" null null))
      (bind _output_get_3 (set `/Game/Blueprints/Food.Mesh Shape` "/Game/Mesh/Mozarella.Mozarella" _returnvalue_3))
      (set `/Game/Blueprints/Food.type` "NewEnumerator5" _returnvalue_3)
      (`StaticMeshComponent.SetStaticMesh` (`/Game/Blueprints/Food.StaticMesh` _returnvalue_3) _output_get_3))
    (:`then_3`
      (bind _returnvalue_4 (`|SpawnActorFromClass` "/Game/Blueprints/Food.Food_C" (`KismetMathLibrary.MakeTransform` (`KismetMathLibrary.RandomPointInBoundingBox` _origin_3 _boxextent_3) (struct :`Roll` 90.0) (1.5 1.5 1.5)) "Undefined" "OverrideRootScale" null null))
      (bind _output_get_4 (set `/Game/Blueprints/Food.Mesh Shape` "/Game/Mesh/Salami.Salami" _returnvalue_4))
      (set `/Game/Blueprints/Food.type` "NewEnumerator1" _returnvalue_4)
      (`StaticMeshComponent.SetStaticMesh` (`/Game/Blueprints/Food.StaticMesh` _returnvalue_4) _output_get_4))
    (:`then_4`
      (bind _returnvalue_5 (`|SpawnActorFromClass` "/Game/Blueprints/Food.Food_C" (`KismetMathLibrary.MakeTransform` (`KismetMathLibrary.RandomPointInBoundingBox` _origin _boxextent) (struct :`Roll` 90.0) (1.5 1.5 1.5)) "Undefined" "OverrideRootScale" null null))
      (bind _output_get_5 (set `/Game/Blueprints/Food.Mesh Shape` "/Game/Mesh/Olive.Olive" _returnvalue_5))
      (set `/Game/Blueprints/Food.type` "NewEnumerator2" _returnvalue_5)
      (`StaticMeshComponent.SetStaticMesh` (`/Game/Blueprints/Food.StaticMesh` _returnvalue_5) _output_get_5))))

(fn `spawn end game`
  (if (>= (`self.spawnTimerEnd`) 0.0)
    (bind _returnvalue (`|SpawnActorFromClass` "/Game/Blueprints/EndGame.EndGame_C" (`KismetMathLibrary.MakeTransform` (0.0 0.0 260.0) (struct :`Roll` 90.0)) "Undefined" "OverrideRootScale" null null))
    (`StaticMeshComponent.SetStaticMesh` (`/Game/Blueprints/EndGame.StaticMesh` _returnvalue) "/Game/Mesh/Endbutton.Endbutton")
    (set `self.spawnTimerEnd` 500.0)
    (set `self.TimeRemaining` (`self.TimerDuration`))))

(fn `Update Game`
  ;[0.5059 1 0.7143] if there is still time remaining continue spawning
  (if (> (`self.TimeRemaining`) 0.0)
    (`|ExecutionSequence`
      (:`then_0`
        (`self.updateTimer`))
      (:`then_1`
        (`self.checkSpawnTimer`)))
    (else
      (set `self.timeUp` true)
      (`self.spawn end game`))))

(fn `updateTimer`
  (set `self.TimeRemaining` (`KismetMathLibrary.FClamp` (- (`self.TimeRemaining`) (`GameplayStatics.GetWorldDeltaSeconds`)) 0.0 100.0))
  (bind _asmrpawn (cast `/Game/Blueprints/MRPawn` (`GameplayStatics.GetPlayerPawn` 0)))
  (`/Game/UI/UIStatus.set timer_text` (`/Game/Blueprints/MRPawn.uistatus` _asmrpawn) (`self.TimeRemaining`)))

(fn `UserConstructionScript`)