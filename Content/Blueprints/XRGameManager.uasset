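; XR game manager for a pizza-topping game: spawns a pizza as the food catcher and random topping Food actors inside SpawnArea.
; Starts an AR session, snapping SpawnArea to detected ceilings and DestroyArea, which destroys overlapping Food, to floors.
; Tick runs countdown and spawn timers, but the zero-clamped countdown never halts spawning and the spawn check passes while its timer is non-negative.
; Status UI creation is unwired.
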(event `self.ReceiveBeginPlay`
  (`ARBlueprintLibrary.StartARSession` "/Game/Config/MainSessionConfig.MainSessionConfig")
  (if (`MicrosoftOpenXRFunctionLibrary.CanDetectPlanes`)
    (`ARBlueprintLibrary.ToggleARCapture` true "SceneUnderstanding")
    (else
      (`ARBlueprintLibrary.ToggleARCapture` true "SpatialMapping")))
  ;[1 1 1] game start
  (set `self.TimeRemaining` (`self.TimerDuration`))
  (set `self.SpawnTimer` (`self.DurationBetweenSpawns`))
  (bind _returnvalue (`|SpawnActorFromClass` "/Game/Blueprints/Pizza.Pizza_C" (`KismetMathLibrary.MakeTransform` (50.0 0.0 0.0) (struct) (0.4 0.4 0.02)) "AlwaysSpawn" "OverrideRootScale" null null))
  (set `self.foodCatcher` _returnvalue))

(event `self.ReceiveTick`
  (params (DeltaSeconds :type "Float (single-precision)"))
  ;[1 1 1] update game
  (`self.UpdateGame`))

(event `self.DestroyArea.OnComponentBeginOverlap`
  (params (OverlappedComponent :type "PrimitiveComponent Object Reference") (OtherActor :type "Actor Object Reference") (OtherComp :type "PrimitiveComponent Object Reference") (OtherBodyIndex :type Integer) (bFromSweep :type Boolean) (SweepResult :type "HitResult Structure (by ref)"))
  (bind _asfood (cast `/Game/Blueprints/Food` OtherActor))
  (`self.K2_DestroyActor` _asfood))

(event `self.ReceiveEndPlay`
  (params (EndPlayReason :type "EEndPlayReason Enum" :default "Destroyed"))
  (`ARBlueprintLibrary.StopARSession`))

(event `self.ARTrackableNotify.OnAddTrackedGeometry`
  (params (TrackedGeometry :type "ARTrackedGeometry Object Reference"))
  (bind _returnvalue (`ARTrackedGeometry.GetUnderlyingMesh` TrackedGeometry))
  (if (`KismetSystemLibrary.IsValid` _returnvalue)
    (switch `EARObjectClassification` (`ARTrackedGeometry.GetObjectClassification` TrackedGeometry)
      (:`Ceiling`
        (`SceneComponent.K2_SetWorldTransform` (`self.SpawnArea`) (`SceneComponent.K2_GetComponentToWorld` _returnvalue) false false))
      (:`Floor`
        (`SceneComponent.K2_SetWorldTransform` (`self.DestroyArea`) (`SceneComponent.K2_GetComponentToWorld` _returnvalue) false false)))))

(event `self.ARTrackableNotify.OnAddTrackedPlane`
  (params (TrackedPlane :type "ARPlaneGeometry Object Reference"))
  (bind _returnvalue (`ARTrackedGeometry.GetUnderlyingMesh` TrackedPlane))
  (bind _returnvalue_2 (`SceneComponent.K2_GetComponentToWorld` _returnvalue))
  (if (`KismetSystemLibrary.IsValid` _returnvalue)
    (switch `EARObjectClassification` (`ARTrackedGeometry.GetObjectClassification` TrackedPlane)
      (:`Ceiling`
        (`SceneComponent.K2_SetWorldTransform` (`self.SpawnArea`) _returnvalue_2 false false))
      (:`Floor`
        (`SceneComponent.K2_SetWorldTransform` (`self.DestroyArea`) _returnvalue_2 false false)))))

(fn `checkSpawnTimer`
  (set `self.SpawnTimer` (- (`self.SpawnTimer`) (`GameplayStatics.GetWorldDeltaSeconds`)))
  (if (>= (`self.SpawnTimer`) 0.0)
    (set `self.SpawnTimer` (`self.DurationBetweenSpawns`))
    (`self.spawn`)))

(fn `spawn`
  (bind (_origin _boxextent) (`KismetSystemLibrary.GetComponentBounds` (`self.SpawnArea`)))
  (bind _returnvalue (`|SpawnActorFromClass` "/Game/Blueprints/Food.Food_C" (`KismetMathLibrary.MakeTransform` (`KismetMathLibrary.RandomPointInBoundingBox` _origin _boxextent) (struct) (0.4 0.4 0.4)) "Undefined" "OverrideRootScale" null null))
  (set `/Game/Blueprints/Food.Mesh Shape` "/Game/Mesh/old/Cheese.Cheese" _returnvalue)
  (`StaticMeshComponent.SetStaticMesh` (`/Game/Blueprints/Food.StaticMesh` _returnvalue) (select `int` (`KismetMathLibrary.RandomIntegerInRange` 0 3) :`0` "/Game/Mesh/old/Cheese.Cheese" :`1` "/Game/Mesh/old/Mozarella.Mozarella" :`2` "/Game/Mesh/old/OLive.OLive" :`3` "/Game/Mesh/old/Salami.Salami" :`4` "/Game/Mesh/old/Tomate.Tomate" :!type "StaticMesh Object Reference")))

(fn `UpdateGame`
  ;[0.5059 1 0.7143] if there is still time remaining continue spawning
  (if (>= (`self.TimeRemaining`) 0.0)
    (`|ExecutionSequence`
      (:`then_0`
        (`self.updateTimer`))
      (:`then_1`
        (`self.checkSpawnTimer`)))))

(fn `updateTimer`
  (set `self.TimeRemaining` (`KismetMathLibrary.FClamp` (- (`self.TimeRemaining`) (`GameplayStatics.GetWorldDeltaSeconds`)) 0.0 100.0)))

(fn `UserConstructionScript`)